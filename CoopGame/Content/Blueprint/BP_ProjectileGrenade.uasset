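; Grenade projectile that explodes when its fuse timer runs out or when something overlaps Sphere2.
; BeginPlay starts the fuse; an overlap calls Explode, clears the timer and destroys Sphere2.
; Explode spawns an explosion emitter, applies radial damage credited to the instigator, and applies radial impulse and force to its own Sphere component only.
; It then destroys that Sphere rather than the actor; a debug radius draw is left disconnected.
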(event `self.ReceiveBeginPlay`
  (bind _returnvalue (`KismetSystemLibrary.K2_SetTimer` self "Explode" (`self.FuseTime`)))
  (set `self.TimerHandle_Fuse` _returnvalue))

(event `Explode`
  (bind _returnvalue (`self.K2_GetActorLocation`))
  (bind _damageradius (`self.DamageRadius`))
  (`GameplayStatics.SpawnEmitterAtLocation` "/Game/WeaponEffects/Explosion/P_Explosion.P_Explosion" _returnvalue (struct) (2.0 2.0 2.0))
  (`GameplayStatics.ApplyRadialDamage` :`BaseDamage` 150.0 :`Origin` _returnvalue :`DamageRadius` _damageradius :`DamageCauser` self :`InstigatedByController` (`self.GetInstigatorController`))
  (`PrimitiveComponent.AddRadialImpulse` (`self.Sphere`) _returnvalue _damageradius 400.0 "RIF_Constant" false)
  (`PrimitiveComponent.AddRadialForce` (`self.Sphere`) _returnvalue _damageradius 400.0 "RIF_Constant" false)
  (`ActorComponent.K2_DestroyComponent` (`self.Sphere`)))

(event `self.Sphere2.OnComponentBeginOverlap`
  (params (OverlappedComponent :type "PrimitiveComponent Object Reference") (OtherActor :type "Actor Object Reference") (OtherComp :type "PrimitiveComponent Object Reference") (OtherBodyIndex :type Integer) (bFromSweep :type Boolean) (SweepResult :type "HitResult Structure (by ref)"))
  (`self.Explode`)
  (`KismetSystemLibrary.K2_ClearAndInvalidateTimerHandle` (`self.TimerHandle_Fuse`))
  (`ActorComponent.K2_DestroyComponent` (`self.Sphere2`)))

(fn `UserConstructionScript`)