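; BP_TrackerBot is a tracker bot Blueprint that scales the volume of its audio with its movement speed.
; Each Tick maps velocity length into a clamped multiplier for AudioComp, so faster movement is louder, and prints that value for debugging.
; An AI move toward the player pawn is present but disconnected, so this graph does not drive movement.
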(event `self.ReceiveBeginPlay`
  ;[1 1 1] Test
)

(event `self.ReceiveTick`
  (params (DeltaSeconds :type "Float (single-precision)"))
  (bind _returnvalue (`KismetMathLibrary.MapRangeClamped` (`KismetMathLibrary.VSize` (`self.GetVelocity`)) 10.0 1000.0 0.1 2.0))
  (`AudioComponent.SetVolumeMultiplier` (`self.AudioComp`) _returnvalue)
  (`KismetSystemLibrary.PrintString` (`KismetStringLibrary.Conv_DoubleToString` _returnvalue) true true (struct :`G` 0.66 :`B` 1.0 :`A` 1.0) 0.0))

(fn `UserConstructionScript`)