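; Bot spawner actor that places a BP_AdvancedAI just above itself at BeginPlay and replaces it each time it dies.
; It binds to the spawned bot's SHealthComponent OnHealthChanged event, and health at or below zero immediately spawns a replacement and binds to it the same way.
; Spawns adjust for collision or are skipped, and nothing here retries a failed spawn.
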(event `self.ReceiveBeginPlay`
  (bind _returnvalue (`self.GetComponentByClass` (`self.SpawnedAI`) "/Script/CoopGame.SHealthComponent"))
  (bind _returnvalue_2 (`|SpawnActorFromClass` "/Game/AI/BP_AdvancedAI.BP_AdvancedAI_C" (`KismetMathLibrary.Conv_VectorToTransform` (+ (`self.K2_GetActorLocation`) (0.0 0.0 50.0))) "AdjustIfPossibleButDontSpawnIfColliding" "OverrideRootScale" null null))
  (set `self.SpawnedAI` _returnvalue_2)
  (`/Engine/EditorBlueprintResources/StandardMacros.IsValid` _returnvalue :!label _label
    (:`Is Valid`
      (add `SHealthComponent.OnHealthChanged` _returnvalue (delegate `OnHealthChanged`)))))

(event `OnHealthChanged`
  (params (HealthComp :type "SHealthComponent Object Reference") (Health :type "Float (double-precision)") (HealthDelta :type "Float (double-precision)") (DamageType :type "DamageType Object Reference") (InstigatedBy :type "Controller Object Reference") (DamageCauser :type "Actor Object Reference"))
  (if (<= Health 0.0)
    (bind _returnvalue (`|SpawnActorFromClass` "/Game/AI/BP_AdvancedAI.BP_AdvancedAI_C" (`KismetMathLibrary.Conv_VectorToTransform` (+ (`self.K2_GetActorLocation`) (0.0 0.0 50.0))) "AdjustIfPossibleButDontSpawnIfColliding" "OverrideRootScale" null null))
    (set `self.SpawnedAI` _returnvalue)
    (goto _label)))

(fn `UserConstructionScript`)